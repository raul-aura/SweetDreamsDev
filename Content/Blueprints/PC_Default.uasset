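; Default player controller that turns Enhanced Input actions into movement, camera and crouch commands for the player's character.
; It adds the input mapping context on BeginPlay, then forwards axis values to the Dream Character's move and camera functions, with camera sensitivity fixed in the graph.
; Crouch is a toggle, using a FlipFlop to alternate Crouch and UnCrouch on player character 0.
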(event `self.ReceiveBeginPlay`
  (`EnhancedInputSubsystemInterface.AddMappingContext` (subsystem `EnhancedInputLocalPlayerSubsystem`) "/Game/Input/InputMapping.InputMapping" 0 (struct)))

(event `EnhancedInput|/Game/Input/IA_CameraHorizontal`
  (params (ActionValue :type "Float (double-precision)") (ElapsedSeconds :type "Float (double-precision)") (TriggeredSeconds :type "Float (double-precision)") (InputAction :type "InputAction Object Reference" :default "/Game/Input/IA_CameraHorizontal.IA_CameraHorizontal"))
  ;[0.2587 0.2587 0.2587] Movement and crouch
  (:`Triggered`
    (`SweetDreamsCharacter.CameraHorizontal` (`self.GetDreamCharacter`) ActionValue 1.0)))

(event `EnhancedInput|/Game/Input/IA_HorizontalAxis`
  (params (ActionValue :type "Float (double-precision)") (ElapsedSeconds :type "Float (double-precision)") (TriggeredSeconds :type "Float (double-precision)") (InputAction :type "InputAction Object Reference" :default "/Game/Input/IA_HorizontalAxis.IA_HorizontalAxis"))
  ;[0.2587 0.2587 0.2587] Movement and crouch
  (:`Triggered`
    (`SweetDreamsCharacter.MoveRight` (`self.GetDreamCharacter`) ActionValue)))

(event `EnhancedInput|/Game/Input/IA_CameraVertical`
  (params (ActionValue :type "Float (double-precision)") (ElapsedSeconds :type "Float (double-precision)") (TriggeredSeconds :type "Float (double-precision)") (InputAction :type "InputAction Object Reference" :default "/Game/Input/IA_CameraVertical.IA_CameraVertical"))
  ;[0.2587 0.2587 0.2587] Movement and crouch
  (:`Triggered`
    (`SweetDreamsCharacter.CameraVertical` (`self.GetDreamCharacter`) ActionValue 1.0)))

(event `EnhancedInput|/Game/Input/IA_VerticalAxis`
  (params (ActionValue :type "Float (double-precision)") (ElapsedSeconds :type "Float (double-precision)") (TriggeredSeconds :type "Float (double-precision)") (InputAction :type "InputAction Object Reference" :default "/Game/Input/IA_VerticalAxis.IA_VerticalAxis"))
  ;[0.2587 0.2587 0.2587] Movement and crouch
  (:`Triggered`
    (`SweetDreamsCharacter.MoveForward` (`self.GetDreamCharacter`) ActionValue)))

(event `EnhancedInput|/Game/Input/IA_Crouch`
  (params (ActionValue :type Boolean) (ElapsedSeconds :type "Float (double-precision)") (TriggeredSeconds :type "Float (double-precision)") (InputAction :type "InputAction Object Reference" :default "/Game/Input/IA_Crouch.IA_Crouch"))
  (bind _returnvalue (`GameplayStatics.GetPlayerCharacter` 0))
  ;[0.2587 0.2587 0.2587] Movement and crouch
  (:`Triggered`
    (`/Engine/EditorBlueprintResources/StandardMacros.FlipFlop`
      (:`A`
        (`Character.Crouch` _returnvalue))
      (:`B`
        (`Character.UnCrouch` _returnvalue)))))

(fn `UserConstructionScript`)