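; Player controller for block editing in a voxel world: left click removes a block, right click places one.
; Both clicks use Raycast, a debug-drawn line trace from player 0's camera, offsetting the hit by its normal to pick the target.
; Removal reaches the DreamScape chunk generator through the ServerRemoveBlock event, while placement calls AddBlock directly with a fixed block ID.
; Kick reasons are printed to screen.
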(event `Key|LeftMouseButton`
  (params (Key :type "Key Structure"))
  (:`Pressed`
    (bind (_location _normal) (`self.Raycast`))
    (`self.Server Remove Block` _location _normal)))

(event `Key|RightMouseButton`
  (params (Key :type "Key Structure"))
  (:`Pressed`
    (bind (_location _normal) (`self.Raycast`))
    (`DreamScapeChunkGenerator.AddBlock` (`DreamScapeChunkGenerator.GetDreamScapeChunkGenerator`) (+ _location _normal) 1)))

(event `Server Remove Block`
  (params (A :type "Vector Structure") (B :type "Vector Structure"))
  (`DreamScapeChunkGenerator.RemoveBlock` (`DreamScapeChunkGenerator.GetDreamScapeChunkGenerator`) (- A B)))

(event `self.OnPlayerKicked`
  (params (KickReason :type "Text (by ref)"))
  (`KismetSystemLibrary.PrintString` (`KismetTextLibrary.Conv_TextToString` KickReason)))

(fn `Raycast`
  (returns (Location :type "Vector Structure") (Normal :type "Vector Structure"))
  (bind _returnvalue (`GameplayStatics.GetPlayerCharacter` 0))
  (bind _returnvalue_2 (`self.GetComponentByClass` _returnvalue "/Script/Engine.CameraComponent"))
  (bind _returnvalue_3 (`SceneComponent.K2_GetComponentLocation` _returnvalue_2))
  (bind _outhit (`KismetSystemLibrary.LineTraceSingle` _returnvalue_3 (+ _returnvalue_3 (* (`KismetMathLibrary.GetForwardVector` (`SceneComponent.K2_GetComponentRotation` _returnvalue_2)) 1400.0)) "TraceTypeQuery1" false (`|MakeArray` _returnvalue :!type "Actor Object Reference") "ForDuration"))
  (bind (_bblockinghit _binitialoverlap _time _distance _location _impactpoint _normal) (`GameplayStatics.BreakHitResult` _outhit))
  (return _location _normal))

(fn `UserConstructionScript`)