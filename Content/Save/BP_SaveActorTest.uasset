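; BP_SaveActorTest is a test actor for the save system that changes a color and saves it to the persistent save.
; It pushes its Color variable into a material parameter collection on BeginPlay.
; ChangeandSaveColor sets Color to a fixed dark red, refreshes the collection, then calls SaveGame on the persistent save object.
; The local and persistent custom data getters are empty stubs.
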(event `self.ReceiveBeginPlay`
  (`self.Event Update Color`))

(event `Event Update Color`
  (`KismetMaterialLibrary.SetVectorParameterValue` "/Game/Save/MatCollection.MatCollection" "Color" (`self.Color`)))

(event `Event Change and Save Color`
  (set `self.Color` (struct :`R` 0.619792 :`A` 1.0))
  (`self.Event Update Color`)
  (`SweetDreamsBPLibrary.SaveGame` (`SweetDreamsBPLibrary.GetPersistentSave`)))

(fn `GetLocalCustomData`
  (returns (ReturnValue :type "Map of Name to String"))
  (return))

(fn `GetPersistentCustomData`
  (returns (ReturnValue :type "Map of Name to String"))
  (return))

(fn `UserConstructionScript`)