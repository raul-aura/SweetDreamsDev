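; BP_INteract is an always-interactable actor that appears to be a test hook for dialogue and inventory.
; On interaction, it looks up the dialogue named "Test", starts it, then prints the name of the first inventory item through PrintDream, without checking that one exists.
; Its interactable name is empty, and its BeginPlay, overlap, Tick and construction logic are unused.
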(event `SweetDreamsInteractInterface.OnInteract`
  (`SweetDreamsDialogueManager.StartDialogue` (`SweetDreamsDialogueManager.FindDialogueByName` "Test") 1.0)
  (`SweetDreamsBPLibrary.PrintDream` (`KismetStringLibrary.Conv_NameToString` (`.ItemName` (break `InventoryItem` (`|GetArrayItem` (`InventoryComponent.GetItems` (`self.Inventory`))))))))

(fn `GetInteractableName`
  (returns (ReturnValue :type Text))
  (return ""))

(fn `IsInteractable`
  (returns (ReturnValue :type Boolean))
  (return true))

(fn `UserConstructionScript`)