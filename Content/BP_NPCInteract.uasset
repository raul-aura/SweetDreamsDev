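; BP_NPCInteract is an interactable NPC Blueprint that appears to be an early test of inventory item adding.
; On interact it adds two of its ItemData to Inventory, then prints the display name of the first inventory item's data through PrintDream.
; It always reports itself interactable and returns an empty interactable name; a count readout is left unconnected.
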(event `SweetDreamsInteractInterface.OnInteract`
  (bind _inventory (`self.Inventory`))
  (`InventoryComponent.AddItem` _inventory (`self.Item Data`) 2 false)
  (`SweetDreamsBPLibrary.PrintDream` (`KismetSystemLibrary.GetDisplayName` (`.ItemData` (break `InventoryItem` (`|GetArrayItem` (`InventoryComponent.GetItems` _inventory)))))))

(fn `GetInteractableName`
  (returns (ReturnValue :type Text))
  (return ""))

(fn `IsInteractable`
  (returns (ReturnValue :type Boolean))
  (return true))

(fn `UserConstructionScript`)